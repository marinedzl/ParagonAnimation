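; LocationBall is a mesh actor that starts with zero color alpha and fades on demand through TriggerFade_Event.
; On BeginPlay it creates a dynamic material instance from the mesh's first material, caches the base color parameter and zeroes its alpha.
; TriggerFade_Event replays a timeline from the start, feeding SetTransparent, which scales only the cached color's alpha and writes it back to the material.
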(event Custom|TriggerFade_Event
  (bind _transparent (Timeline|FadeTimeline PlayFromStart)
    (:Update
      (CallFunction|SetTransparent _transparent))))

(event EventBeginPlay
  (CallFunction|CreateDynamicMaterial))

(event Collision|EventActorBeginOverlap
  (params (OtherActor :type Actor%20Object%20Reference)))

(event EventTick
  (params (DeltaSeconds :type Float%20%28single-precision%29)))

(fn ConstructionScript)

(fn CreateDynamicMaterial
  (bind _staticmeshcomponent (Variables|Debug|GetStaticMeshComponent))
  (bind _returnvalue (Rendering|Material|CreateDynamicMaterialInstance _staticmeshcomponent 0 (Rendering|Material|GetMaterial _staticmeshcomponent 0) "None" :!class /Script/Engine.PrimitiveComponent))
  (bind _output_get (Variables|Default|SetDynamicMaterialInstance _returnvalue))
  (bind _returnvalue_2 (Rendering|Material|GetVectorParameterValue _output_get (Variables|Default|GetBaseColorParamName) :!class /Script/Engine.MaterialInstanceDynamic))
  (Variables|Default|SetBaseColor _returnvalue_2)
  (CallFunction|SetTransparent 0.0))

(fn SetTransparent
  (params (Value :type Float%20%28single-precision%29))
  (Rendering|Material|SetVectorParameterValue (Variables|Default|GetDynamicMaterialInstance) (Variables|Default|GetBaseColorParamName) (* (Utilities|Struct|MakeLinearColor 1.0 1.0 1.0 Value) (Variables|Default|GetBaseColor)) :!class /Script/Engine.MaterialInstanceDynamic))